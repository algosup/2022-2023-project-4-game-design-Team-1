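; ThePlayer is the playable character, with mouse look, keyboard movement, sprinting and rock throwing.
; Movement follows the control rotation's yaw, and sprint press and release swap the walk speed between sprint and normal values.
; Throwing uses up one rock from RockAmount, spawns a RockBP at ObjectREF's location, and launches its Box at fixed speed along the line from the player to that spawn point.
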(event Input|ActionEvents|InputActionKeyboard-Sprint
  (params (Key :type Key%20Structure :default "None"))
  ;[1 1 1] Sprint
  (:Pressed
    (CallFunction|StartSprint))
  (:Released
    (CallFunction|StopSprint)))

(event Input|ActionEvents|InputActionKeyboard-Throw
  (params (Key :type Key%20Structure :default "None"))
  (:Pressed
    (if (!= (Variables|Default|GetRock%20Amount) 0)
      (bind _result (Math|Integer|DecrementInt (Variables|Default|GetRock%20Amount))
        (:%20%20
          (Variables|Default|SetRock%20Amount _result)
          (bind _returnvalue (Game|SpawnActorfromClass "/Game/Blueprints/RockBP.RockBP_C" (Math|Transform|MakeTransform (Transformation|GetWorldLocation (Variables|Default|GetObject%20REF)) (Transformation|GetWorldRotation (Variables|Collision|GetCapsuleComponent)) "1,1,1") "Undefined" 0 0))
          (Physics|SetPhysicsLinearVelocity (Variables|/Game/Blueprints/RockBP.RockBP_C|GetBox _returnvalue) (* (Math|Vector|GetUnitDirection(Vector) (Transformation|GetActorLocation) (Transformation|GetActorLocation _returnvalue)) 1e+03) false "None"))))))

(event Input|AxisEvents|InputAxisKeyboard-Forward/Backward
  (params (AxisValue :type Float%20%28single-precision%29))
  ;[1 1 1] Keyboard - Input
  (Pawn|Input|AddMovementInput self (Math|Vector|GetForwardVector (Math|Rotator|MakeRotator 0.0 0.0 (.Yaw (Math|Rotator|BreakRotator (Pawn|GetControlRotation self :!class /Script/Engine.Pawn))))) AxisValue false))

(event Input|AxisEvents|InputAxisKeyboard-Right/Left
  (params (AxisValue :type Float%20%28single-precision%29))
  ;[1 1 1] Keyboard - Input
  (Pawn|Input|AddMovementInput self (Math|Vector|GetRightVector (Math|Rotator|MakeRotator 0.0 0.0 (.Yaw (Math|Rotator|BreakRotator (Pawn|GetControlRotation self :!class /Script/Engine.Pawn))))) AxisValue false))

(event Input|AxisEvents|InputAxisMouseLookLeft/Right
  (params (AxisValue :type Float%20%28single-precision%29))
  ;[1 1 1] Mouse - Input
  (Pawn|Input|AddControllerYawInput self AxisValue))

(event Input|AxisEvents|InputAxisMouseLookUp/Down
  (params (AxisValue :type Float%20%28single-precision%29))
  ;[1 1 1] Mouse - Input
  (Pawn|Input|AddControllerPitchInput self AxisValue))

(fn ConstructionScript)

(fn StartSprint
  (Variables|/Script/Engine.CharacterMovementComponent|SetMaxWalkSpeed (Variables|Character|GetCharacterMovement) (Variables|Default|GetSprintSpeed)))

(fn StopSprint
  (Variables|/Script/Engine.CharacterMovementComponent|SetMaxWalkSpeed (Variables|Character|GetCharacterMovement) (Variables|Default|GetWalkSpeed)))