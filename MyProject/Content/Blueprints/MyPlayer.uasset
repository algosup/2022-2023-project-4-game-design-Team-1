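; MyPlayer is a player Character Blueprint that handles mouse look, keyboard movement and sprinting.
; Mouse axes drive controller pitch and yaw, while movement axes follow the forward and right vectors of the control rotation's yaw alone.
; Sprint press and release call functions that switch CharacterMovement's max walk speed between sprint and walk values.
; StartCrouch and StopCrouch are empty stubs with no input bound to them.
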(event Input|ActionEvents|InputActionKeyboard-Sprint
  (params (Key :type Key%20Structure :default "None"))
  (:Pressed
    (CallFunction|StartSprint))
  (:Released
    (CallFunction|StopSprint)))

(event Input|AxisEvents|InputAxisKeyboard-Forward/Backward
  (params (AxisValue :type Float%20%28single-precision%29))
  ;[1 1 1] Keyboard - Input
  (Pawn|Input|AddMovementInput self (Math|Vector|GetForwardVector (Math|Rotator|MakeRotator 0.0 0.0 (.Yaw (Math|Rotator|BreakRotator (Pawn|GetControlRotation self :!class /Script/Engine.Pawn))))) AxisValue false))

(event Input|AxisEvents|InputAxisKeyboard-Right/Left
  (params (AxisValue :type Float%20%28single-precision%29))
  ;[1 1 1] Keyboard - Input
  (Pawn|Input|AddMovementInput self (Math|Vector|GetRightVector (Math|Rotator|MakeRotator 0.0 0.0 (.Yaw (Math|Rotator|BreakRotator (Pawn|GetControlRotation self :!class /Script/Engine.Pawn))))) AxisValue false))

(event Input|AxisEvents|InputAxisMouseLookLeft/Right
  (params (AxisValue :type Float%20%28single-precision%29))
  ;[1 1 1] Mouse - Input
  (Pawn|Input|AddControllerYawInput self AxisValue))

(event Input|AxisEvents|InputAxisMouseLookUp/Down
  (params (AxisValue :type Float%20%28single-precision%29))
  ;[1 1 1] Mouse - Input
  (Pawn|Input|AddControllerPitchInput self AxisValue))

(fn ConstructionScript)

(fn StartSprint
  (Variables|/Script/Engine.CharacterMovementComponent|SetMaxWalkSpeed (Variables|Character|GetCharacterMovement) (Variables|Default|GetSprintSpeed)))

(fn StopSprint
  (Variables|/Script/Engine.CharacterMovementComponent|SetMaxWalkSpeed (Variables|Character|GetCharacterMovement) (Variables|Default|GetWalkSpeed)))

(fn StartCrouch)

(fn StopCrouch)