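; RockBP is a rock the player can collect, which also makes noise when it hits something.
; Player overlap opens a Gate so the Interact key increments RockAmount on ThePlayer and destroys the rock.
; End overlap closes the Gate only when the cast to ThePlayer fails.
; Its first hit on anything except the player plays a sound and reports AI-audible noise instigated by the player.
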(event OnComponentBeginOverlap(Interactcollision)
  (params (OverlappedComponent :type Primitive%20Component%20Object%20Reference) (OtherActor :type Actor%20Object%20Reference) (OtherComp :type Primitive%20Component%20Object%20Reference) (OtherBodyIndex :type Integer) (bFromSweep :type Boolean) (SweepResult :type Hit%20Result%20Structure%20%28by%20ref%29))
  (bind _asthe_player (Utilities|Casting|CastToThePlayer OtherActor))
  (Utilities|FlowControl|Gate true) ; enters at Open
)

(event OnComponentEndOverlap(Interactcollision)
  (params (OverlappedComponent :type Primitive%20Component%20Object%20Reference) (OtherActor :type Actor%20Object%20Reference) (OtherComp :type Primitive%20Component%20Object%20Reference) (OtherBodyIndex :type Integer))
  (Utilities|Casting|CastToThePlayer OtherActor
    (:CastFailed
      (Utilities|FlowControl|Gate true) ; enters at Close
    )))

(event Collision|EventHit
  (params (MyComp :type Primitive%20Component%20Object%20Reference) (Other :type Actor%20Object%20Reference) (OtherComp :type Primitive%20Component%20Object%20Reference) (bSelfMoved :type Boolean) (HitLocation :type Vector :default "0, 0, 0") (HitNormal :type Vector :default "0, 0, 0") (NormalImpulse :type Vector :default "0, 0, 0") (Hit :type Hit%20Result%20Structure%20%28by%20ref%29))
  (bind _returnvalue (Game|GetPlayerCharacter 0))
  (bind _returnvalue_2 (Transformation|GetActorLocation))
  (if (!= Other _returnvalue)
    (Utilities|FlowControl|DoOnce false
      (:Completed
        (Audio|PlaySoundatLocation "/Game/SoundsEffect/RockCue.RockCue" _returnvalue_2 "0, 0, 0" 1.0 1.0 0.0 0 0 0)
        (Class|AISenseHearing|ReportNoiseEvent _returnvalue_2 1.0 _returnvalue 5e+02 "None")))))

(event EventBeginPlay
  (Input|EnableInput (Game|GetPlayerController 0)))

(event Input|ActionEvents|InputActionKeyboard-Interact
  (params (Key :type Key%20Structure :default "None"))
  (:Pressed
    (Utilities|FlowControl|Gate true
      (:Exit
        (bind _result (Math|Integer|IncrementInt (Variables|/Game/Blueprints/ThePlayer.ThePlayer_C|GetRock%20Amount (stale OnComponentBeginOverlap(Interactcollision) _asthe_player)))
          (:%20%20
            (Variables|/Game/Blueprints/ThePlayer.ThePlayer_C|SetRock%20Amount (stale OnComponentBeginOverlap(Interactcollision) _asthe_player) _result)
            (Actor|DestroyActor)))))))

(fn ConstructionScript)