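; BP_PressedPuzzle is a step-on code puzzle that opens a linked Door when the player overlaps pads in the correct order.
; The construction script spawns a spaced row of flat meshes, one per CorrectCode character, each under a trigger box tagged with a RandomCode character.
; Player overlaps append that tag to InputCode, which AddCode checks by substring, clearing on mismatch and messaging the Door on a full match.
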(event EventBeginPlay)

(event Collision|EventActorBeginOverlap
  (params (OtherActor :type Actor%20Object%20Reference)))

(event EventTick
  (params (DeltaSeconds :type Float%20%28single-precision%29)))

(fn ConstructionScript
  (for _index (range 0 (- (Utilities|String|Len (Variables|Default|GetCorrectCode)) 1))
    (bind _returnvalue (AddComponent|AddStaticMeshComponent false (Math|Transform|MakeTransform (Math|Vector|MakeVector (Math|Conversions|ToFloat(Integer) (* _index (Math|Float|Truncate (Variables|Default|GetSpacing)))) 0.0 0.0) "0, 0, 0" "1.500000,1.500000,0.100000")))
    (bind _returnvalue_2 (AddComponent|AddBoxComponent false (Math|Transform|MakeTransform (+ (Variables|/Script/Engine.SceneComponent|GetRelativeLocation _returnvalue) "0,0.000000,50.000000") "0, 0, 0" "1.500000,1.500000,1.500000")))
    (Variables|/Script/Engine.ActorComponent|SetComponentTags _returnvalue_2 (Utilities|Array|MakeArray (Utilities|String|StringToName (Utilities|String|GetSubstring (Variables|Default|GetRandomCode) _index))))
    (Collision|BindEventtoOnComponentBeginOverlap _returnvalue_2 (EventDispatchers|CreateEvent :!event BPPressedPuzzleAutoGenFunc))))

(fn BPPressedPuzzleAutoGenFunc
  (params (OverlappedComponent :type Primitive%20Component%20Object%20Reference) (OtherActor :type Actor%20Object%20Reference) (OtherComp :type Primitive%20Component%20Object%20Reference) (OtherBodyIndex :type Integer) (bFromSweep :type Boolean) (SweepResult :type Hit%20Result%20Structure%20%28by%20ref%29))
  (Utilities|Casting|CastToThePlayer OtherActor)
  (CallFunction|AddCode (Utilities|String|ToString(Name) (Utilities|Array|Get(acopy) (Variables|/Script/Engine.ActorComponent|GetComponentTags OverlappedComponent))))
  (return))

(fn AddCode
  (params (Add :type String))
  (bind _output_get (Variables|Default|SetInputCode (Utilities|String|Append (Variables|Default|GetInputCode) Add)))
  (Development|PrintString _output_get)
  (Development|PrintString (Utilities|String|GetSubstring (Variables|Default|GetCorrectCode) (stale _index) (Variables|Default|GetNum)) true true "(R=1.000000,G=0.172212,B=0.589166,A=1.000000)")
  (if (Utilities|Enum|Equal(Enum) (Utilities|String|GetSubstring (Variables|Default|GetCorrectCode) (stale _index) (Variables|Default|GetNum)) (Utilities|String|GetSubstring (Variables|Default|GetInputCode) (stale _index) (Variables|Default|GetNum)))
    (Math|Integer|IncrementInt (Variables|Default|GetNum)
      (:%20%20
        (if (== (Utilities|String|Len (Variables|Default|GetCorrectCode)) (Utilities|String|Len (Variables|Default|GetInputCode)))
          (if (Utilities|Enum|Equal(Enum) (Variables|Default|GetCorrectCode) (Variables|Default|GetInputCode))
            (Class|PuzzleInterface|OpenDoor(Message) (Variables|Default|GetDoor))
            (Variables|Default|SetInputCode "")
            (else
              (Variables|Default|SetInputCode ""))))))
    (else
      (Variables|Default|SetNum 1)
      (Variables|Default|SetInputCode ""))))

(fn BPPressedPuzzleAutoGenFunc1
  (params (OverlappedComponent :type Primitive%20Component%20Object%20Reference) (OtherActor :type Actor%20Object%20Reference) (OtherComp :type Primitive%20Component%20Object%20Reference) (OtherBodyIndex :type Integer) (bFromSweep :type Boolean) (SweepResult :type Hit%20Result%20Structure%20%28by%20ref%29)))