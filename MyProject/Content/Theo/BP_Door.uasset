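; BP_Door is a door actor that slides from its starting location to an end location when opened.
; BeginPlay stores the start location, and the OpenDoor_1 event enables actor Tick.
; Tick accumulates time and linearly interpolates the position over RotationTime, which serves as the move duration despite its name.
; Tick disables itself once that time elapses, with no closing or timer reset logic.
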(event Custom|Open%20Door_1
  (Actor|Tick|SetActorTickEnabled true))

(event EventTick
  (params (DeltaSeconds :type Float%20%28single-precision%29))
  (Variables|Default|SetCurrent%20Time (+ DeltaSeconds (Variables|Default|GetCurrent%20Time)))
  (Transformation|SetActorLocation (Math|Vector|Lerp(Vector) (Variables|Default|GetStart%20Location) (Variables|Default|GetEnd%20Location) (/ (Variables|Default|GetCurrent%20Time) (Variables|Default|GetRotation%20Time))) false false)
  (if (>= (Variables|Default|GetCurrent%20Time) (Variables|Default|GetRotation%20Time))
    (Actor|Tick|SetActorTickEnabled false)))

(event EventBeginPlay
  (Variables|Default|SetStart%20Location (Transformation|GetActorLocation)))

(fn ConstructionScript)