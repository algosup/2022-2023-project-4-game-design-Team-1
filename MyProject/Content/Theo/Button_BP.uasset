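; Interactable button Blueprint that animates a press and plays a rock sound, with no other effect triggered in this file.
; An overlap box opens and closes a Gate for ThePlayer, so the keyboard interact input only works in range.
; The press runs two chained timelines, lerping the button's relative transform to an offset position cached at BeginPlay, then reversing it back out.
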(event OnComponentBeginOverlap(Box)
  (params (OverlappedComponent :type Primitive%20Component%20Object%20Reference) (OtherActor :type Actor%20Object%20Reference) (OtherComp :type Primitive%20Component%20Object%20Reference) (OtherBodyIndex :type Integer) (bFromSweep :type Boolean) (SweepResult :type Hit%20Result%20Structure%20%28by%20ref%29))
  ;[1 1 1] Button Interaction
  (Utilities|Casting|CastToThePlayer OtherActor)
  (Utilities|FlowControl|Gate true) ; enters at Open
)

(event OnComponentEndOverlap(Box)
  (params (OverlappedComponent :type Primitive%20Component%20Object%20Reference) (OtherActor :type Actor%20Object%20Reference) (OtherComp :type Primitive%20Component%20Object%20Reference) (OtherBodyIndex :type Integer))
  ;[1 1 1] Button Interaction
  (Utilities|Casting|CastToThePlayer OtherActor)
  (Utilities|FlowControl|Gate true) ; enters at Close
)

(event EventBeginPlay
  (bind _button (Variables|Default|GetButton))
  (bind _returnvalue (Transformation|GetRelativeTransform _button))
  (Variables|Default|Setout_position (Math|Transform|MakeTransform (.location _returnvalue) (.rotation _returnvalue) (.scale _returnvalue)))
  (Variables|Default|Setin_position (Math|Transform|MakeTransform (- (.location _returnvalue) "0,-10.000000, 0") (.rotation _returnvalue) (.scale _returnvalue)))
  (Input|EnableInput (Game|GetPlayerController 0)))

(event Input|ActionEvents|InputActionKeyboard-InteractButton
  (params (Key :type Key%20Structure :default "None"))
  ;[1 1 1] Button Interaction
  (:Pressed
    (Utilities|FlowControl|Gate true
      (:Exit
        ;[1 1 1] Button moving animation
        (|ButtonAnimation)))))

(fn ConstructionScript)