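; RockBP is a rock the player can collect, which also makes noise when it strikes something.
; Overlapping InteractCollision as ThePlayer1 opens a gate letting Pick Up input increment RockAmount and destroy the rock.
; The gate closes only when the end-overlap cast to ThePlayer1 fails, so the player leaving does not close it.
; The first non-player hit plays RockCue and reports a long-range noise event instigated by the player.
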(event OnComponentBeginOverlap(Interactcollision)
  (params (OverlappedComponent :type Primitive%20Component%20Object%20Reference) (OtherActor :type Actor%20Object%20Reference) (OtherComp :type Primitive%20Component%20Object%20Reference) (OtherBodyIndex :type Integer) (bFromSweep :type Boolean) (SweepResult :type Hit%20Result%20Structure%20%28by%20ref%29))
  ;[1 1 1] Grab a rock
  (bind _asthe_player_1 (Utilities|Casting|CastToThePlayer1 OtherActor))
  (Utilities|FlowControl|Gate true) ; enters at Open
)

(event OnComponentEndOverlap(Interactcollision)
  (params (OverlappedComponent :type Primitive%20Component%20Object%20Reference) (OtherActor :type Actor%20Object%20Reference) (OtherComp :type Primitive%20Component%20Object%20Reference) (OtherBodyIndex :type Integer))
  ;[1 1 1] Grab a rock
  (Utilities|Casting|CastToThePlayer1 OtherActor
    (:CastFailed
      (Utilities|FlowControl|Gate true) ; enters at Close
    )))

(event Collision|EventHit
  (params (MyComp :type Primitive%20Component%20Object%20Reference) (Other :type Actor%20Object%20Reference) (OtherComp :type Primitive%20Component%20Object%20Reference) (bSelfMoved :type Boolean) (HitLocation :type Vector :default "0, 0, 0") (HitNormal :type Vector :default "0, 0, 0") (NormalImpulse :type Vector :default "0, 0, 0") (Hit :type Hit%20Result%20Structure%20%28by%20ref%29))
  (bind _returnvalue (Game|GetPlayerCharacter 0))
  ;[1 1 1] Sound Effect
  (if (!= Other _returnvalue)
    (Utilities|FlowControl|DoOnce false
      (:Completed
        (Audio|PlaySoundatLocation "/Game/MindMaze/SoundsEffect/RockCue.RockCue" HitLocation "0, 0, 0" 1.0 1.0 0.0 0 0 0)
        (bind _output_get (Variables|Default|SetRockLocation HitLocation))
        (Class|AISenseHearing|ReportNoiseEvent _output_get 1.0 _returnvalue 1e+04 "None")))))

(event EventBeginPlay
  (Input|EnableInput (Game|GetPlayerController 0)))

(event Input|ActionEvents|InputActionKeyboard-PickUp
  (params (Key :type Key%20Structure :default "None"))
  ;[1 1 1] Grab a rock
  (:Pressed
    (Utilities|FlowControl|Gate true
      (:Exit
        (bind _result (Math|Integer|IncrementInt (Variables|/Game/MindMaze/Blueprints/ThePlayer1.ThePlayer1_C|GetRock%20Amount (stale OnComponentBeginOverlap(Interactcollision) _asthe_player_1)))
          (:%20%20
            (Variables|/Game/MindMaze/Blueprints/ThePlayer1.ThePlayer1_C|SetRock%20Amount (stale OnComponentBeginOverlap(Interactcollision) _asthe_player_1) _result)
            (Actor|DestroyActor)))))))

(fn ConstructionScript)