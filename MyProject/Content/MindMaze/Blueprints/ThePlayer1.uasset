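; Player character for MindMaze, handling mouse look, yaw-relative movement, sprinting, pausing and rock throwing.
; Sprint swaps the max walk speed while held, and the pause input toggles a lazily created menu widget along with game pause, cursor and input mode.
; Throwing spends a rock from the count, spawns it at a reference component and launches it along the direction from the player to that spawn point.
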(event Input|ActionEvents|InputActionKeyboard-Sprint
  (params (Key :type Key%20Structure :default "None"))
  ;[1 1 1] Sprint
  (:Pressed
    (CallFunction|StartSprint))
  (:Released
    (CallFunction|StopSprint)))

(event Input|ActionEvents|InputActionKeyboard-Throw
  (params (Key :type Key%20Structure :default "None"))
  ;[1 1 1] Throw
  (:Pressed
    (if (!= (Variables|Default|GetRock%20Amount) 0)
      (bind _result (Math|Integer|DecrementInt (Variables|Default|GetRock%20Amount))
        (:%20%20
          (Variables|Default|SetRock%20Amount _result)
          (bind _returnvalue (Game|SpawnActorfromClass "/Game/MindMaze/Blueprints/RockBP.RockBP_C" (Math|Transform|MakeTransform (Transformation|GetWorldLocation (Variables|Default|GetObject%20REF)) (Transformation|GetWorldRotation (Variables|Collision|GetCapsuleComponent)) "1,1,1") "Undefined" 0 0))
          (Physics|SetPhysicsLinearVelocity (Variables|/Game/MindMaze/Blueprints/RockBP.RockBP_C|GetBox _returnvalue) (* (Math|Vector|GetUnitDirection(Vector) (Transformation|GetActorLocation) (Transformation|GetActorLocation _returnvalue)) 7e+02) false "None"))))))

(event Input|ActionEvents|InputActionPauseGame
  (params (Key :type Key%20Structure :default "None"))
  (bind _returnvalue (Game|GetPlayerController 0))
  ;[1 1 1] Pause / Unpause Game
  (:Pressed
    (Utilities|IsValid (Variables|Default|GetPause%20Menu%20REF)
      (:Is%20Valid
        _)
      (:Is%20Not%20Valid
        (bind _returnvalue_2 (UserInterface|CreateWidget "/Game/Alex/Pause_Menu/PauseMenuWidget.PauseMenuWidget_C"))
        (Variables|Default|SetPause%20Menu%20REF _returnvalue_2)))
    (if (Game|IsGamePaused)
      (Widget|RemovefromParent (Variables|Default|GetPause%20Menu%20REF))
      (Game|SetGamePaused false)
      (Variables|/Script/Engine.PlayerController|SetbShowMouseCursor _returnvalue false)
      (Input|SetInputModeGameOnly _returnvalue)
      (else
        (UserInterface|Viewport|AddtoViewport (Variables|Default|GetPause%20Menu%20REF) 0)
        (Game|SetGamePaused true)
        (Variables|/Script/Engine.PlayerController|SetbShowMouseCursor _returnvalue true)
        (Input|SetInputModeGameandUI _returnvalue (Variables|Default|GetPause%20Menu%20REF) "LockInFullscreen" false)))))

(event Input|AxisEvents|InputAxisKeyboard-Forward/Backward
  (params (AxisValue :type Float%20%28single-precision%29))
  ;[1 1 1] Keyboard - Input
  (Pawn|Input|AddMovementInput self (Math|Vector|GetForwardVector (Math|Rotator|MakeRotator 0.0 0.0 (.Yaw (Math|Rotator|BreakRotator (Pawn|GetControlRotation self :!class /Script/Engine.Pawn))))) AxisValue false))

(event Input|AxisEvents|InputAxisKeyboard-Right/Left
  (params (AxisValue :type Float%20%28single-precision%29))
  ;[1 1 1] Keyboard - Input
  (Pawn|Input|AddMovementInput self (Math|Vector|GetRightVector (Math|Rotator|MakeRotator 0.0 0.0 (.Yaw (Math|Rotator|BreakRotator (Pawn|GetControlRotation self :!class /Script/Engine.Pawn))))) AxisValue false))

(event Input|AxisEvents|InputAxisMouseLookLeft/Right
  (params (AxisValue :type Float%20%28single-precision%29))
  ;[1 1 1] Mouse - Input
  (Pawn|Input|AddControllerYawInput self AxisValue))

(event Input|AxisEvents|InputAxisMouseLookUp/Down
  (params (AxisValue :type Float%20%28single-precision%29))
  ;[1 1 1] Mouse - Input
  (Pawn|Input|AddControllerPitchInput self AxisValue))

(fn ConstructionScript)

(fn StartSprint
  (Variables|/Script/Engine.CharacterMovementComponent|SetMaxWalkSpeed (Variables|Character|GetCharacterMovement) (Variables|Default|GetSprintSpeed)))

(fn StopSprint
  (Variables|/Script/Engine.CharacterMovementComponent|SetMaxWalkSpeed (Variables|Character|GetCharacterMovement) (Variables|Default|GetWalkSpeed)))